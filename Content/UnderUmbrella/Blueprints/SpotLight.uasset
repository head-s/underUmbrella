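; SpotLight Blueprint that publishes where its spot light beam lands to the SpotLightParam material parameter collection.
; On each Box component hit event, it runs a debug-drawn Visibility trace along the light's forward axis, slightly past the attenuation radius.
; The impact point becomes the HotSpot vector.
; Radius approximates the cone footprint as clamped impact distance times outer cone angle in radians; Tick is empty.
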(event `self.ReceiveTick`
  (params (DeltaSeconds :type "Float (single-precision)")))

(event `self.Box.OnComponentHit`
  (params (OtherActor :type "Actor Object Reference") (OtherComp :type "PrimitiveComponent Object Reference") (NormalImpulse :type "Vector Structure") (Hit :type "HitResult Structure (by ref)"))
  (bind _spotlight (`self.SpotLight`))
  (bind _returnvalue (`SceneComponent.K2_GetComponentLocation` _spotlight))
  (bind _attenuationradius (`PointLightComponent.AttenuationRadius` _spotlight))
  (bind _outhit (`KismetSystemLibrary.LineTraceSingle` :`Start` _returnvalue :`End` (+ _returnvalue (`KismetMathLibrary.GreaterGreater_VectorRotator` (`KismetMathLibrary.MakeVector` (+ _attenuationradius 50.0)) (`SceneComponent.K2_GetComponentRotation` _spotlight))) :`TraceChannel` "TraceTypeQuery1" :`DrawDebugType` "ForOneFrame"))
  (bind (_bblockinghit _binitialoverlap _time _location _impactpoint) (`GameplayStatics.BreakHitResult` _outhit))
  (`KismetMaterialLibrary.SetVectorParameterValue` "/Game/UnderUmbrella/Materials/SpotLightParam.SpotLightParam" "HotSpot" (`KismetMathLibrary.Conv_VectorToLinearColor` _impactpoint))
  (`KismetMaterialLibrary.SetScalarParameterValue` "/Game/UnderUmbrella/Materials/SpotLightParam.SpotLightParam" "Radius" (* (`KismetMathLibrary.FClamp` (`KismetMathLibrary.VSize` (- _impactpoint (`SceneComponent.K2_GetComponentLocation` (`self.SpotLight`)))) 0.0 _attenuationradius) (`KismetMathLibrary.DegreesToRadians` (`SpotLightComponent.OuterConeAngle` _spotlight)))))

(fn `UserConstructionScript`)